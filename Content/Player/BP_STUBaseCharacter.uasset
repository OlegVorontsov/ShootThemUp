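; Base player character that handles mouse wheel camera zoom by changing the spring arm length within min and max height limits.
; A flag picks between an instant step per scroll and a smooth slide.
; The smooth slide runs a looping timer that moves the arm in small increments until one step distance is covered, ignoring further scroll input until it finishes.
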(event `self.ReceiveTick`
  (params (DeltaSeconds :type "Float (single-precision)")))

(event `InputAxisKey|MouseWheelAxis`
  (params (AxisValue :type "Float (single-precision)"))
  (if (`self.SlideCameraWithSmooth`)
    (`self.CameraSlideSmooth` AxisValue)
    (else
      (`self.CameraSlide` AxisValue))))

(fn `CameraSlide`
  (params (Value :type "Float (double-precision)"))
  (bind _springarm (`self.SpringArm`))
  (bind _heightcamerachangedistance (`self.HeightCameraChangeDistance`))
  (bind _targetarmlength (`SpringArmComponent.TargetArmLength` _springarm))
  (bind _returnvalue (- _targetarmlength _heightcamerachangedistance))
  (bind _returnvalue_2 (+ _targetarmlength _heightcamerachangedistance))
  (if (!= Value 0.0)
    (if (< Value 0.0)
      (if (> (`self.HeightCameraMax`) _returnvalue_2)
        (set `SpringArmComponent.TargetArmLength` _returnvalue_2 _springarm))
      (elif (< (`self.HeightCameraMin`) _returnvalue)
        (set `SpringArmComponent.TargetArmLength` _returnvalue _springarm)))))

(fn `CameraSlideSmooth`
  (params (Value :type "Float (double-precision)"))
  (bind _heightcamerachangedistance (`self.HeightCameraChangeDistance`))
  (bind _targetarmlength (`SpringArmComponent.TargetArmLength` (`self.SpringArm`)))
  (if (`self.SlideDone`)
    (if (!= Value 0.0)
      (if (< Value 0.0)
        (if (>= (`self.HeightCameraMax`) (+ _targetarmlength _heightcamerachangedistance))
          (set `self.SlideUp` true)
          (set `self.SlideDone` false :!label _label)
          (bind _returnvalue (`KismetSystemLibrary.K2_SetTimer` null "CameraSlideSmoothTick" (`self.TimerStep`) true))
          (set `self.SlideTimer` _returnvalue))
        (elif (<= (`self.HeightCameraMin`) (- _targetarmlength _heightcamerachangedistance))
          (set `self.SlideUp` false)
          (goto _label))))))

(fn `CameraSlideSmoothTick`
  (bind _heightcamerachangeslidestepdistance (`self.HeightCameraChangeSlideStepDistance`))
  (bind _springarm (`self.SpringArm`))
  (bind _targetarmlength (`SpringArmComponent.TargetArmLength` _springarm))
  (bind _output_get (set `self.CurrentSlideDistance` (+ (`self.CurrentSlideDistance`) _heightcamerachangeslidestepdistance)))
  (set `SpringArmComponent.TargetArmLength` (select `bool` (`self.SlideUp`) :`false` (- _targetarmlength _heightcamerachangeslidestepdistance) :`true` (+ _targetarmlength _heightcamerachangeslidestepdistance)) _springarm)
  (if (>= _output_get (`self.HeightCameraChangeDistance`))
    (set `self.CurrentSlideDistance` 0.0)
    (set `self.SlideDone` true)
    (`KismetSystemLibrary.K2_ClearAndInvalidateTimerHandle` (`self.SlideTimer`))))

(fn `UserConstructionScript`)